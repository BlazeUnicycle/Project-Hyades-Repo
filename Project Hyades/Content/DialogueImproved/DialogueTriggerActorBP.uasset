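; Actor blueprint that starts a dialogue scene at its own location from its dialogue data table.
; ActorDialogue passes the table to SpawnDialogue, which spawns a SceneTemplateBP at the actor's transform, stores it as the current scene, registers itself as the start actor and initiates the scene.
; An IsScenePlaying flag, set here but never cleared here, blocks repeat spawns while a scene plays.
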(event Custom|Actor%20Dialogue
  (CallFunction|SpawnDialogue (Variables|Default|GetDialogueDataTable)))

(event Custom|Spawn%20Dialogue
  (params (DataTable :type Data%20Table%20Object%20Reference))
  (if (not (Variables|Default|GetIsScenePlaying))
    (Variables|Default|SetIsScenePlaying true)
    (bind _returnvalue (Game|SpawnActorfromClass "/Game/DialogueImproved/SceneTemplateBP.SceneTemplateBP_C" (Transformation|GetActorTransform) "Undefined" 0 0))
    (bind _output_get (Variables|Default|SetCurrent%20Scene _returnvalue))
    (Variables|/Game/DialogueImproved/SceneTemplateBP.SceneTemplateBP_C|SetSceneStartActor _output_get self)
    (Default|InitiateNewScene _output_get DataTable)))

(event EventBeginPlay)

(event Collision|EventActorBeginOverlap
  (params (OtherActor :type Actor%20Object%20Reference)))

(event EventTick
  (params (DeltaSeconds :type Float%20%28single-precision%29)))

(fn ConstructionScript)