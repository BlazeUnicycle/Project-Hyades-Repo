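; SceneTemplateBP is a dialogue scene actor that plays a DataTable of lines through a DisplayDialogue widget.
; InitiateNewScene caches the table's rows, and PlayLine shows each one's text and speaker name.
; After a short delay, choice rows create a DisplayChoices widget, while others let the NextLine input advance.
; Past the last row, it removes the widget, clears IsScenePlaying on SceneStartActor and destroys itself.
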(event Custom|Initiate%20New%20Scene
  (params (CurrentScene :type Data%20Table%20Object%20Reference))
  (bind _outrownames (DataTable|GetDataTableRowNames CurrentScene))
  (for _array_element _outrownames
    (bind _returnvalue (Utilities|GetDataTableRow CurrentScene _array_element)
      (:then
        (Utilities|Array|Add (Variables|Default|GetArrayOfRows) _returnvalue))))
  (bind _returnvalue_2 (UserInterface|CreateWidget "/Game/DialogueImproved/DisplayDialogue.DisplayDialogue_C"))
  (bind _output_get (Variables|Default|SetDisplayDialogue%20Widget _returnvalue_2))
  (UserInterface|Viewport|AddtoViewport _output_get 0)
  (CallFunction|PlayLine))

(event Custom|Play%20Line
  (bind _arrayofrows (Variables|Default|GetArrayOfRows))
  (bind _currentrow (Variables|Default|GetCurrentRow))
  (bind _displaydialogue_widget (Variables|Default|GetDisplayDialogue%20Widget))
  (bind _output (Utilities|Array|Get(acopy) _arrayofrows _currentrow))
  (bind (_speaker _expression _text _charhorizontal _ischoice_) (Utilities|Struct|BreakDialogueStruct _output))
  (Variables|Default|SetIsRowFinished false)
  (if (>= (Variables|Default|GetCurrentRow) (Utilities|Array|Length (Variables|Default|GetArrayOfRows)))
    (CallFunction|DestroyDialogueScene)
    (else
      (Utilities|IsValid _displaydialogue_widget
        (:Is%20Valid
          (Variables|/Game/DialogueImproved/DisplayDialogue.DisplayDialogue_C|SetText _displaydialogue_widget (Utilities|Text|ToText(String) _text))
          (Rendering|Components|TextRender|SetText (Variables|/Game/DialogueImproved/DisplayDialogue.DisplayDialogue_C|GetSpeakerName _displaydialogue_widget) (Utilities|Text|ToText(String) (Utilities|String|EnumtoString _speaker)))
          (Variables|Default|SetIsPlayerChoice _ischoice_)
          (Utilities|FlowControl|Delay 0.2)
          (if (Variables|Default|GetIsPlayerChoice)
            (UserInterface|CreateWidget "/Game/DialogueImproved/DisplayChoices.DisplayChoices_C")
            (else
              (Variables|Default|SetIsRowFinished true))))))))

(event Custom|Destroy%20Dialogue%20Scene
  (Widget|RemovefromParent (Variables|Default|GetDisplayDialogue%20Widget))
  (Variables|/Game/DialogueImproved/DialogueTriggerActorBP.DialogueTriggerActorBP_C|SetIsScenePlaying (Variables|Default|GetSceneStartActor) false)
  (Actor|DestroyActor))

(event EventBeginPlay
  (Input|EnableInput (Game|GetPlayerController 0)))

(event Collision|EventActorBeginOverlap
  (params (OtherActor :type Actor%20Object%20Reference)))

(event EventTick
  (params (DeltaSeconds :type Float%20%28single-precision%29)))

(event Input|ActionEvents|InputActionNextLine
  (params (Key :type Key%20Structure :default "None"))
  (:Pressed
    (if (Variables|Default|GetIsRowFinished)
      (Math|Integer|IncrementInt (Variables|Default|GetCurrentRow)
        (:%20%20
          (CallFunction|PlayLine))))))

(fn ConstructionScript)