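; Trigger actor that starts a dialogue when the first-person character overlaps it.
; On overlap it passes its DialogueDataTable to the level's DialogueTriggerActorBP, found by class, via SpawnDialogue.
; The IsDoOnce flag routes the overlap through a DoOnce for one-time triggering.
; An unconnected leftover branch would spawn a SceneTemplateBP and start the scene directly, but never runs.
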(event EventBeginPlay)

(event EventTick
  (params (DeltaSeconds :type Float%20%28single-precision%29)))

(event Collision|EventActorBeginOverlap
  (params (OtherActor :type Actor%20Object%20Reference))
  (Utilities|Casting|CastToFirstPersonCharacter OtherActor)
  (if (Variables|Default|GetisDoOnce?)
    (Utilities|FlowControl|DoOnce false
      (:Completed
        _)))
  (bind _returnvalue (Actor|GetActorOfClass "/Game/DialogueImproved/DialogueTriggerActorBP.DialogueTriggerActorBP_C"))
  (Default|SpawnDialogue _returnvalue (Variables|Default|GetDialogueDataTable)))

(fn ConstructionScript)